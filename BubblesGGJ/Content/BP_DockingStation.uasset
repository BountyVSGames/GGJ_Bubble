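; Docking station that switches the player pawn's element (Copper, Carbon, Clear or Light) when it enters the charge trigger.
; The construction script previews the element's material; BeginPlay labels it and caches player gravity and velocity.
; Overlap swaps sphere material and element components (Clear only deactivates Carbon) and plays a sound.
; The sphere snaps to the trigger for a second with gravity off, then reattaches as cached values return.
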(event OnComponentBeginOverlap(Docking_ChargeTrigger)
  (params (OverlappedComponent :type Primitive%20Component%20Object%20Reference) (OtherActor :type Actor%20Object%20Reference) (OtherComp :type Primitive%20Component%20Object%20Reference) (OtherBodyIndex :type Integer) (bFromSweep :type Boolean) (SweepResult :type Hit%20Result%20Structure%20%28by%20ref%29))
  (bind _asbp_pawn (Utilities|Casting|CastToBP_Pawn OtherActor))
  (CallFunction|ChangeElement _asbp_pawn)
  (Audio|PlaySoundatLocation "/Game/Audio/connecting.connecting" (Transformation|GetActorLocation self) "0, 0, 0" 1.0 1.0 0.0 0 0 0 0)
  (CallFunction|ConnectPlayer))

(event Custom|ConnectPlayer
  (CallFunction|ToggleGravity false)
  (bind _asbp_pawn (Utilities|Casting|CastToBP_Pawn (Game|GetPlayerCharacter 0)))
  (bind _returnvalue (Transformation|AttachComponentToComponent (Variables|/Game/Blueprints/BP_Pawn.BP_Pawn_C|GetSphere _asbp_pawn) (Variables|Default|GetDocking_ChargeTrigger) "None" "SnapToTarget" "SnapToTarget" "KeepWorld" false))
  (if _returnvalue
    (Default|OnDocking _asbp_pawn)
    (Variables|/Game/Blueprints/BPC_PlayerMovement.BPC_PlayerMovement_C|SetIsDocked (Variables|/Game/Blueprints/BP_Pawn.BP_Pawn_C|GetBPC_PlayerMovement _asbp_pawn) true)
    (Utilities|FlowControl|Delay 1.0)
    (CallFunction|ToggleGravity true)
    (Transformation|AttachComponentToComponent (Variables|/Game/Blueprints/BP_Pawn.BP_Pawn_C|GetSphere _asbp_pawn) (Variables|/Script/Engine.Character|GetCapsuleComponent _asbp_pawn) "None" "SnapToTarget" "SnapToTarget" "KeepWorld" false)
    (Variables|/Game/Blueprints/BPC_PlayerMovement.BPC_PlayerMovement_C|SetIsDocked (Variables|/Game/Blueprints/BP_Pawn.BP_Pawn_C|GetBPC_PlayerMovement _asbp_pawn) false)))

(event Custom|Toggle%20Gravity
  (params (Gravity :type Boolean))
  (if Gravity
    (bind _asbp_pawn (Utilities|Casting|CastToBP_Pawn (Game|GetPlayerCharacter 0)))
    (Variables|/Script/Engine.CharacterMovementComponent|SetGravityScale (Variables|/Script/Engine.Character|GetCharacterMovement _asbp_pawn) (Variables|Default|GetCurrentGravityScale))
    (Variables|/Script/Engine.MovementComponent|SetVelocity (Variables|/Script/Engine.Character|GetCharacterMovement _asbp_pawn) (Variables|Default|GetCurrentVelocity))
    (else
      (bind _asbp_pawn_2 (Utilities|Casting|CastToBP_Pawn (Game|GetPlayerCharacter 0)))
      (Variables|/Script/Engine.CharacterMovementComponent|SetGravityScale (Variables|/Script/Engine.Character|GetCharacterMovement _asbp_pawn_2) 0.0)
      (Variables|/Script/Engine.MovementComponent|SetVelocity (Variables|/Script/Engine.Character|GetCharacterMovement _asbp_pawn_2) "0, 0, 0"))))

(event EventBeginPlay
  (CallFunction|DisplayElementText)
  (bind _asbp_pawn (Utilities|Casting|CastToBP_Pawn (Game|GetPlayerCharacter 0)))
  (Variables|Default|SetCurrentGravityScale (Variables|/Script/Engine.CharacterMovementComponent|GetGravityScale (Variables|/Script/Engine.Character|GetCharacterMovement _asbp_pawn)))
  (Variables|Default|SetCurrentVelocity (Variables|/Script/Engine.MovementComponent|GetVelocity (Variables|/Script/Engine.Character|GetCharacterMovement _asbp_pawn))))

(event Collision|EventActorBeginOverlap
  (params (OtherActor :type Actor%20Object%20Reference)))

(event EventTick
  (params (DeltaSeconds :type Float%20%28single-precision%29)))

(fn ConstructionScript
  (bind _elementdisplay (Variables|Default|GetElementDisplay))
  (switch Utilities|FlowControl|Switch|SwitchonE_Elements (Variables|Default|GetElements)
    (:NewEnumerator1
      (Rendering|Material|SetMaterial _elementdisplay 0 "/Game/M_Copper.M_Copper"))
    (:NewEnumerator3
      (Rendering|Material|SetMaterial _elementdisplay 0 "/Game/M_Carbon.M_Carbon"))
    (:NewEnumerator4
      (Rendering|Material|SetMaterial _elementdisplay 0 "/Game/M_Clear.M_Clear"))
    (:NewEnumerator5
      (Rendering|Material|SetMaterial _elementdisplay 0 "/Game/M_LightDockingStation.M_LightDockingStation"))))

(fn ChangeElement
  (params (Player :type BP%20Pawn%20Object%20Reference))
  (bind _sphere (Variables|/Game/Blueprints/BP_Pawn.BP_Pawn_C|GetSphere Player))
  (switch Utilities|FlowControl|Switch|SwitchonE_Elements (Variables|Default|GetElements)
    (:NewEnumerator1
      (Rendering|Material|SetMaterial _sphere 0 "/Game/M_Copper.M_Copper")
      (Components|Activation|SetActive (Variables|/Game/Blueprints/BP_Pawn.BP_Pawn_C|GetBPC_Carbon Player) false false)
      (Components|Activation|SetActive (Variables|/Game/Blueprints/BP_Pawn.BP_Pawn_C|GetBPC_Clear Player) false false)
      (Components|Activation|SetActive (Variables|/Game/Blueprints/BP_Pawn.BP_Pawn_C|GetBPC_Copper Player) true false))
    (:NewEnumerator3
      (Rendering|Material|SetMaterial _sphere 0 "/Game/M_Carbon.M_Carbon")
      (Components|Activation|SetActive (Variables|/Game/Blueprints/BP_Pawn.BP_Pawn_C|GetBPC_Copper Player) false false)
      (Components|Activation|SetActive (Variables|/Game/Blueprints/BP_Pawn.BP_Pawn_C|GetBPC_Clear Player) false false)
      (Components|Activation|SetActive (Variables|/Game/Blueprints/BP_Pawn.BP_Pawn_C|GetBPC_Carbon Player) true false))
    (:NewEnumerator4
      (Rendering|Material|SetMaterial _sphere 0 "/Game/M_Clear.M_Clear")
      (Components|Activation|SetActive (Variables|/Game/Blueprints/BP_Pawn.BP_Pawn_C|GetBPC_Carbon Player) false false))
    (:NewEnumerator5
      (Rendering|Material|SetMaterial _sphere 0 "/Game/M_Light.M_Light")
      (Components|Activation|SetActive (Variables|/Game/Blueprints/BP_Pawn.BP_Pawn_C|GetBPC_Carbon Player) false false)
      (Components|Activation|SetActive (Variables|/Game/Blueprints/BP_Pawn.BP_Pawn_C|GetBPC_Copper Player) false false)
      (Components|Activation|SetActive (Variables|/Game/Blueprints/BP_Pawn.BP_Pawn_C|GetBPC_Clear Player) false false)
      (Components|Activation|SetActive (Variables|/Game/Blueprints/BP_Pawn.BP_Pawn_C|GetBPC_Light Player) true false))))

(fn DisplayElementText
  (Rendering|Components|TextRender|SetText (Variables|Default|GetElementText) (Utilities|Text|ToText(String) (Utilities|String|EnumtoString (Variables|Default|GetElements)))))