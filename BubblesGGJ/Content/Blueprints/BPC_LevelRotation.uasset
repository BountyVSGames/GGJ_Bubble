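; BPC_LevelRotation is an actor component apparently meant to tilt the level from player horizontal input, but currently unfinished.
; BeginPlay binds to BP_Pawn's horizontal movement event and caches the owner, its start rotation and the player.
; The Horizontal handler is empty; disconnected logic would smooth input into clamped owner pitch and shift custom gravity.
; RotateActorAroundPoint only draws a debug line to the computed orbit position, without moving anything.
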(event Custom|Horizontal
  (params (ActionValue :type Vector%202D%20Structure)))

(event EventBeginPlay
  (bind _returnvalue (Actor|GetActorOfClass "/Game/Blueprints/BP_Pawn.BP_Pawn_C"))
  (EventDispatchers|BindEventtoHorizontalMovement _returnvalue (EventDispatchers|CreateEvent :!event Custom|Horizontal))
  (bind _output_get (Variables|Default|SetOwner (Components|GetOwner)))
  (Variables|Default|SetStartRotation (Transformation|GetActorRotation _output_get))
  (bind _returnvalue_2 (Actor|GetActorOfClass "/Game/Blueprints/BP_Pawn.BP_Pawn_C"))
  (Variables|Default|SetPlayer _returnvalue_2))

(fn RotateActorAroundPoint
  (params (Angle :type Float%20%28double-precision%29) (PointToRotateAround :type Vector) (AxisToRotateAround :type Vector))
  (Rendering|Debug|DrawDebugLine :LineStart (Transformation|GetActorLocation (Variables|Default|GetPlayer)) :LineEnd (+ (Math|Vector|RotateVectorAroundAxis (- (Transformation|GetActorLocation (Variables|Default|GetOwner)) PointToRotateAround) Angle AxisToRotateAround) PointToRotateAround) :Duration 1e+01)
  (return))