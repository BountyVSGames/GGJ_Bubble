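; BPC_PlayerMovement is a BP_Pawn component that handles camera rotation, gravity direction and sideways dashes.
; It binds to the owner's horizontal movement and trigger events on BeginPlay.
; Horizontal input smoothly drives camera world pitch, then roll is clamped and the camera's negated up vector becomes the CustomGravityNode movement component's gravity direction.
; Triggers dash the pawn along the camera's right axis, with debug print and line calls left in.
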(event Custom|CameraMovement
  (params (ActionValue :type Vector%202D%20Structure))
  (bind _owner (Variables|Default|GetOwner))
  (bind _camera (Variables|/Game/Blueprints/BP_Pawn.BP_Pawn_C|GetCamera _owner))
  (bind _returnvalue (Transformation|GetWorldRotation _camera))
  (Variables|Default|SetCurrentSpeed (Math|Interpolation|FInterpTo (Variables|Default|GetCurrentSpeed) (* (.X (Math|Vector2D|BreakVector2D ActionValue)) (Variables|Default|GetSpeed)) (Utilities|Time|GetWorldDeltaSeconds) 5.0))
  (Transformation|AddWorldRotation _camera (Math|Rotator|MakeRotator 0.0 (Variables|Default|GetCurrentSpeed) 0.0) false false)
  (Development|PrintString (Utilities|String|ToString(Float) (.roll _returnvalue)))
  (Transformation|SetWorldRotation _camera (Math|Rotator|MakeRotator (Math|Float|Clamp(Float) (.roll _returnvalue) -1.3e+02 1.3e+02) (.pitch _returnvalue) (.yaw _returnvalue)) false false)
  (Class|CustomGravityNode|SetGravDirection (.AsCustom%20Gravity%20Node (Utilities|Casting|CastToCustomGravityNode (Variables|/Script/Engine.Character|GetCharacterMovement (Variables|Default|GetOwner)))) (* (Math|Vector|GetUpVector (Transformation|GetWorldRotation _camera)) -1.0)))

(event Custom|RightTrigger
  (params (ActionValue :type Float%20%28double-precision%29))
  (bind _owner (Variables|Default|GetOwner))
  (Rendering|Debug|DrawDebugLine :LineStart (Transformation|GetActorLocation _owner) :Duration 1e+02)
  (Default|DashTrigger (Variables|Default|GetOwner) (* (Math|Vector|GetRightVector (Variables|/Game/Blueprints/BP_Pawn.BP_Pawn_C|GetCamera _owner)) (Variables|Default|GetDashDistance))))

(event Custom|LeftTrigger
  (params (ActionValue :type Float%20%28double-precision%29))
  (Default|DashTrigger (Variables|Default|GetOwner) (* (Math|Vector|GetRightVector (Variables|/Game/Blueprints/BP_Pawn.BP_Pawn_C|GetCamera (Variables|Default|GetOwner))) (* (Variables|Default|GetDashDistance) -1.0))))

(event EventBeginPlay
  (bind _asbp_pawn (Utilities|Casting|CastToBP_Pawn (Components|GetOwner)))
  (Variables|Default|SetOwner _asbp_pawn)
  (EventDispatchers|BindEventtoHorizontalMovement _asbp_pawn (EventDispatchers|CreateEvent :!event Custom|CameraMovement))
  (EventDispatchers|BindEventtoLeftTrigger _asbp_pawn (EventDispatchers|CreateEvent :!event Custom|LeftTrigger))
  (EventDispatchers|BindEventtoRighTrigger _asbp_pawn (EventDispatchers|CreateEvent :!event Custom|RightTrigger)))

(event EventTick
  (params (DeltaSeconds :type Float%20%28single-precision%29)))