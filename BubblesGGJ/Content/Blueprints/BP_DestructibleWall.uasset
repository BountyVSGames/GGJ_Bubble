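; Destructible wall actor that spawns a Niagara destruction effect and destroys itself.
; When the player pawn overlaps its Box, the effect spawns at the pawn's Sphere location using the wall's rotation.
; A separate CE_DestroyWall event spawns the same effect at the wall's own location before destroying the actor.
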(event OnComponentBeginOverlap(Box)
  (params (OverlappedComponent :type Primitive%20Component%20Object%20Reference) (OtherActor :type Actor%20Object%20Reference) (OtherComp :type Primitive%20Component%20Object%20Reference) (OtherBodyIndex :type Integer) (bFromSweep :type Boolean) (SweepResult :type Hit%20Result%20Structure%20%28by%20ref%29))
  (bind _returnvalue (Game|Player|GetPlayerPawn 0))
  (if (== _returnvalue OtherActor)
    (Niagara|SpawnSystematLocation "/Game/Blueprints/NS_DestroyWall.NS_DestroyWall" (Transformation|GetWorldLocation (Variables|/Game/Blueprints/BP_Pawn.BP_Pawn_C|GetSphere (.AsBP%20Pawn (Utilities|Casting|CastToBP_Pawn _returnvalue)))) (Transformation|GetWorldRotation (Variables|Default|GetWall)))
    (Actor|DestroyActor)))

(event Custom|CE_DestroyWall
  (bind _wall (Variables|Default|GetWall))
  (Niagara|SpawnSystematLocation "/Game/Blueprints/NS_DestroyWall.NS_DestroyWall" (Transformation|GetWorldLocation _wall) (Transformation|GetWorldRotation _wall))
  (Actor|DestroyActor))

(event EventBeginPlay)

(event Collision|EventActorBeginOverlap
  (params (OtherActor :type Actor%20Object%20Reference)))

(event EventTick
  (params (DeltaSeconds :type Float%20%28single-precision%29)))

(fn ConstructionScript)