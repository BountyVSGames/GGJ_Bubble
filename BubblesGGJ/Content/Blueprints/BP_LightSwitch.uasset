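; BP_LightSwitch is a switch actor that toggles registered darkness objects when the pawn begins overlapping it.
; AssignDarkness fills DarknessRef, and each toggle plays or reverses every entry's LightSwitch while swapping the Sphere's on/off material.
; BeginPlay binds to the pawn's interact event.
; LightSwitchTrigger reuses the toggle when OverlappingWithPawn is true, but the node setting that flag is disconnected, leaving that path and Tick's debug print inactive.
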(event Custom|LightSwitchTrigger
  (if (Variables|Default|GetOverlappingWithPawn)
    (if (Variables|Default|GetLightState)
      (for _array_element (Variables|Default|GetDarknessRef)
        (Components|Timeline|PlayfromStart (Variables|/Game/Blueprints/BP_Darkness.BP_Darkness_C|GetLightSwitch _array_element))
        (Rendering|Material|SetMaterial (Variables|Default|GetSphere) 0 (Variables|Default|GetLightsOffMaterial)))
      (Variables|Default|SetLightState false)
      (else
        (for _array_element_2 (Variables|Default|GetDarknessRef)
          (Components|Timeline|ReversefromEnd (Variables|/Game/Blueprints/BP_Darkness.BP_Darkness_C|GetLightSwitch _array_element_2))
          (Rendering|Material|SetMaterial (Variables|Default|GetSphere) 0 (Variables|Default|GetLightsOnMaterial)))
        (Variables|Default|SetLightState true)))))

(event Custom|AssignDarkness
  (params (NewParam :type BP%20Darkness%20Object%20Reference))
  (Utilities|Array|Add (Variables|Default|GetDarknessRef) NewParam))

(event EventBeginPlay
  (bind _returnvalue (Actor|GetActorOfClass "/Game/Blueprints/BP_Pawn.BP_Pawn_C"))
  (EventDispatchers|BindEventtoInteract _returnvalue (EventDispatchers|CreateEvent :!event Custom|LightSwitchTrigger)))

(event Collision|EventActorBeginOverlap
  (params (OtherActor :type Actor%20Object%20Reference))
  (Utilities|Casting|CastToBP_Pawn OtherActor)
  (if (Variables|Default|GetLightState)
    (for _array_element (Variables|Default|GetDarknessRef)
      (Components|Timeline|PlayfromStart (Variables|/Game/Blueprints/BP_Darkness.BP_Darkness_C|GetLightSwitch _array_element))
      (Rendering|Material|SetMaterial (Variables|Default|GetSphere) 0 (Variables|Default|GetLightsOffMaterial)))
    (Variables|Default|SetLightState false)
    (else
      (for _array_element_2 (Variables|Default|GetDarknessRef)
        (Components|Timeline|ReversefromEnd (Variables|/Game/Blueprints/BP_Darkness.BP_Darkness_C|GetLightSwitch _array_element_2))
        (Rendering|Material|SetMaterial (Variables|Default|GetSphere) 0 (Variables|Default|GetLightsOnMaterial)))
      (Variables|Default|SetLightState true))))

(event EventTick
  (params (DeltaSeconds :type Float%20%28single-precision%29))
  (if (Variables|Default|GetOverlappingWithPawn)
    (Development|PrintString "Hello")))

(event Collision|EventActorEndOverlap
  (params (OtherActor :type Actor%20Object%20Reference))
  (Utilities|Casting|CastToBP_Pawn OtherActor)
  (if (Variables|Default|GetOverlappingWithPawn)
    (Variables|Default|SetOverlappingWithPawn false)))

(fn ConstructionScript)