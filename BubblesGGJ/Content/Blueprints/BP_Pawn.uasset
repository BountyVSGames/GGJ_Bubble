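; BP_Pawn is a player pawn that turns Enhanced Input into jumps and dispatcher calls, and supports a dash.
; BeginPlay adds the IM_Player mapping context, then move, left, right and interact inputs are relayed through dispatchers while jump is handled directly.
; DashTrigger plays a timeline that applies a swept world-transform delta scaled toward EndPoint each update, and OnDocking stops it.
; Disconnected leftovers include sphere velocity clamping, a thud sound and alternative dash movement.
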(event OnComponentBeginOverlap(CapsuleComponent)
  (params (OverlappedComponent :type Primitive%20Component%20Object%20Reference) (OtherActor :type Actor%20Object%20Reference) (OtherComp :type Primitive%20Component%20Object%20Reference) (OtherBodyIndex :type Integer) (bFromSweep :type Boolean) (SweepResult :type Hit%20Result%20Structure%20%28by%20ref%29)))

(event Custom|DashTrigger
  (params (EndPoint :type Vector))
  (bind _newtrack_0 (Timeline|Dash PlayFromStart)
    (:Update
      (Development|PrintString (Utilities|String|ToString(Float) _newtrack_0))
      (Class|Actor|AddActorWorldTransform self (Math|Transform|MakeTransform (Math|Vector|Lerp(Vector) "0, 0, 0" EndPoint _newtrack_0) "0, 0, 0" "1.000000,1.000000,1.000000") true false))))

(event Custom|OnDocking
  (bind _newtrack_0 (Timeline|Dash Stop)
    (:Update
      (Development|PrintString (Utilities|String|ToString(Float) _newtrack_0))
      (Class|Actor|AddActorWorldTransform self (Math|Transform|MakeTransform (Math|Vector|Lerp(Vector) "0, 0, 0" (stale Custom|DashTrigger EndPoint) _newtrack_0) "0, 0, 0" "1.000000,1.000000,1.000000") true false))))

(event Input|EnhancedActionEvents|EnhancedInputActionIA_Left
  (params (ActionValue :type Float%20%28double-precision%29) (ElapsedSeconds :type Float%20%28double-precision%29) (TriggeredSeconds :type Float%20%28double-precision%29) (InputAction :type Input%20Action%20Object%20Reference :default "/Game/Input/IA_Left.IA_Left"))
  (Default|CallLeftTrigger ActionValue))

(event Input|EnhancedActionEvents|EnhancedInputActionIA_Jump
  (params (ActionValue :type Boolean) (ElapsedSeconds :type Float%20%28double-precision%29) (TriggeredSeconds :type Float%20%28double-precision%29) (InputAction :type Input%20Action%20Object%20Reference :default "/Game/Input/IA_Jump.IA_Jump"))
  (Character|Jump))

(event Input|EnhancedActionEvents|EnhancedInputActionIA_Move
  (params (ActionValue :type Vector%202D%20Structure) (ElapsedSeconds :type Float%20%28double-precision%29) (TriggeredSeconds :type Float%20%28double-precision%29) (InputAction :type Input%20Action%20Object%20Reference :default "/Game/Input/IA_Move.IA_Move"))
  (Default|CallHorizontalMovement ActionValue))

(event Input|EnhancedActionEvents|EnhancedInputActionIA_Right
  (params (ActionValue :type Float%20%28double-precision%29) (ElapsedSeconds :type Float%20%28double-precision%29) (TriggeredSeconds :type Float%20%28double-precision%29) (InputAction :type Input%20Action%20Object%20Reference :default "/Game/Input/IA_Right.IA_Right"))
  (Default|CallRighTrigger ActionValue))

(event Input|EnhancedActionEvents|EnhancedInputActionIA_Interact
  (params (ActionValue :type Boolean) (ElapsedSeconds :type Float%20%28double-precision%29) (TriggeredSeconds :type Float%20%28double-precision%29) (InputAction :type Input%20Action%20Object%20Reference :default "/Game/Input/IA_Interact.IA_Interact"))
  (:Started
    (Default|CallInteract)))

(event EventTick
  (params (DeltaSeconds :type Float%20%28single-precision%29)))

(event EventBeginPlay
  (bind _returnvalue (Game|GetPlayerController 0))
  (Utilities|IsValid _returnvalue
    (:Is%20Valid
      (Input|AddMappingContext (PlayerController|LocalPlayerSubsystems|GetEnhancedInputLocalPlayerSubsystem _returnvalue) "/Game/Input/IM_Player.IM_Player" 0 "(bIgnoreAllPressedKeysUntilRelease=True,bForceImmediately=False,bNotifyUserSettings=False)"))))

(fn ConstructionScript)